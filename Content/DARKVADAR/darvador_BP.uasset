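; Darvador actor that flips its Runningman component 180 degrees whenever one of nine row flags on the floor turns true.
; Every Tick it looks up Floor_bp actors and polls the row flags on the first one found.
; Each row has its own DoOnce, reset while that flag is false, so the component rotates once per activation rather than every frame.
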(event `self.ReceiveTick`
  (params (DeltaSeconds :type "Float (single-precision)"))
  (bind _outactors (`GameplayStatics.GetAllActorsOfClass` "/Game/floor_bp.floor_bp_C"))
  (`|ExecutionSequence`
    (:`then_0`
      (bind _output (`|GetArrayItem` _outactors))
      (if (== (`/Game/floor_bp.1st row hit` _output) true)
        (`/Engine/EditorBlueprintResources/StandardMacros.DoOnce` false :!label _label
          (:`Completed`
            (`SceneComponent.K2_AddWorldRotation` (`self.runningman`) (struct :`Yaw` 180.0) false false)))
        (else
          (goto _label :!via `Reset`))))
    (:`then_1`
      (if (== (`/Game/floor_bp.2nd row hit` _output) true)
        (`/Engine/EditorBlueprintResources/StandardMacros.DoOnce` false :!label _label_2
          (:`Completed`
            (`SceneComponent.K2_AddWorldRotation` (`self.runningman`) (struct :`Yaw` 180.0) false false)))
        (else
          (goto _label_2 :!via `Reset`))))
    (:`then_2`
      (if (== (`/Game/floor_bp.3rd row hit` _output) true)
        (`/Engine/EditorBlueprintResources/StandardMacros.DoOnce` false :!label _label_3
          (:`Completed`
            (`SceneComponent.K2_AddWorldRotation` (`self.runningman`) (struct :`Yaw` 180.0) false false)))
        (else
          (goto _label_3 :!via `Reset`))))
    (:`then_3`
      (if (== (`/Game/floor_bp.4th row hit` _output) true)
        (`/Engine/EditorBlueprintResources/StandardMacros.DoOnce` false :!label _label_4
          (:`Completed`
            (`SceneComponent.K2_AddWorldRotation` (`self.runningman`) (struct :`Yaw` 180.0) false false)))
        (else
          (goto _label_4 :!via `Reset`))))
    (:`then_4`
      (if (== (`/Game/floor_bp.5th row` _output) true)
        (`/Engine/EditorBlueprintResources/StandardMacros.DoOnce` false :!label _label_5
          (:`Completed`
            (`SceneComponent.K2_AddWorldRotation` (`self.runningman`) (struct :`Yaw` 180.0) false false)))
        (else
          (goto _label_5 :!via `Reset`))))
    (:`then_5`
      (if (== (`/Game/floor_bp.6th row` _output) true)
        (`/Engine/EditorBlueprintResources/StandardMacros.DoOnce` false :!label _label_6
          (:`Completed`
            (`SceneComponent.K2_AddWorldRotation` (`self.runningman`) (struct :`Yaw` 180.0) false false)))
        (else
          (goto _label_6 :!via `Reset`))))
    (:`then_6`
      (if (== (`/Game/floor_bp.7th row` _output) true)
        (`/Engine/EditorBlueprintResources/StandardMacros.DoOnce` false :!label _label_7
          (:`Completed`
            (`SceneComponent.K2_AddWorldRotation` (`self.runningman`) (struct :`Yaw` 180.0) false false)))
        (else
          (goto _label_7 :!via `Reset`))))
    (:`then_7`
      (if (== (`/Game/floor_bp.8th row` _output) true)
        (`/Engine/EditorBlueprintResources/StandardMacros.DoOnce` false :!label _label_8
          (:`Completed`
            (`SceneComponent.K2_AddWorldRotation` (`self.runningman`) (struct :`Yaw` 180.0) false false)))
        (else
          (goto _label_8 :!via `Reset`))))
    (:`then_8`
      (if (== (`/Game/floor_bp.9th row` _output) true)
        (`/Engine/EditorBlueprintResources/StandardMacros.DoOnce` false :!label _label_9
          (:`Completed`
            (`SceneComponent.K2_AddWorldRotation` (`self.runningman`) (struct :`Yaw` 180.0) false false)))
        (else
          (goto _label_9 :!via `Reset`))))))

(fn `UserConstructionScript`)