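; Snake actor that plays a squash animation on its static mesh when the SnakeShake1 flag on Camera_bp1 is set.
; Tick looks up the first Camera_bp1 actor every frame and plays a timeline while the flag is true.
; The timeline curve lerps the mesh's relative Y scale, and a short delay after it finishes clears the flag.
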(event `self.ReceiveTick`
  (params (DeltaSeconds :type "Float (single-precision)"))
  (bind _outactors (`GameplayStatics.GetAllActorsOfClass` "/Game/camera_bp1.camera_bp1_C"))
  (bind _output (`|GetArrayItem` _outactors))
  (if (== (`/Game/camera_bp1.snake shake1` _output) true)
    (bind (_direction _newtrack_0222) (`Timeline|Timeline_0`)
      (:`Update`
        (`SceneComponent.SetRelativeScale3D` (`self.StaticMesh`) (`KismetMathLibrary.VLerp` (5.0 4.0 5.0) (5.0 3.0 5.0) _newtrack_0222)))
      (:`Finished`
        (`KismetSystemLibrary.Delay` 0.5)
        (set `/Game/camera_bp1.snake shake1` false _output)))))

(fn `UserConstructionScript`)