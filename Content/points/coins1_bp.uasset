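; A coin pickup that spins and awards points to either of two player characters, darvador_BP or darvador_BP2.
; Tick rotates the mesh by a fixed step per frame, independent of delta time.
; Each player has its own trigger, which plays a sound and calls PointsP1xxl or PointsP2xxl on all Camera_bp1 actors.
; The coin destroys itself after a short delay, with no guard against repeat overlaps meanwhile.
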(event `self.ReceiveTick`
  (params (DeltaSeconds :type "Float (single-precision)"))
  (`SceneComponent.K2_AddLocalRotation` (`self.coin mesh`) (struct :`Yaw` 1.0) false false))

(event `self.coin trigger1.OnComponentBeginOverlap`
  (params (OverlappedComponent :type "PrimitiveComponent Object Reference") (OtherActor :type "Actor Object Reference") (OtherComp :type "PrimitiveComponent Object Reference") (OtherBodyIndex :type Integer) (bFromSweep :type Boolean) (SweepResult :type "HitResult Structure (by ref)"))
  (cast `/Game/DARKVADAR/darvador_BP` OtherActor)
  (`GameplayStatics.PlaySound2D` "/Game/points/coin_sound.coin_sound" 1.0 1.0 0.0 null null)
  (bind _outactors (`GameplayStatics.GetAllActorsOfClass` "/Game/camera_bp1.camera_bp1_C"))
  (`/Game/camera_bp1.points p1xxl` _outactors)
  (`KismetSystemLibrary.Delay` 0.2)
  (`self.K2_DestroyActor`))

(event `self.coin trigger2.OnComponentBeginOverlap`
  (params (OverlappedComponent :type "PrimitiveComponent Object Reference") (OtherActor :type "Actor Object Reference") (OtherComp :type "PrimitiveComponent Object Reference") (OtherBodyIndex :type Integer) (bFromSweep :type Boolean) (SweepResult :type "HitResult Structure (by ref)"))
  (cast `/Game/DARKVADAR/darvador_BP2` OtherActor)
  (`GameplayStatics.PlaySound2D` "/Game/points/coin_sound.coin_sound" 1.0 1.0 0.0 null null)
  (bind _outactors (`GameplayStatics.GetAllActorsOfClass` "/Game/camera_bp1.camera_bp1_C"))
  (`/Game/camera_bp1.points p2xxl` _outactors)
  (`KismetSystemLibrary.Delay` 0.2)
  (`self.K2_DestroyActor`))

(fn `NewFunction_0`)

(fn `UserConstructionScript`)