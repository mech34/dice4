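; Floor actor for a two-player game that tracks which of nine rows each player touches and detects when either player wins.
; Separate overlap volumes per player (Row for darvador_BP, Box for darvador_BP2) pulse that row's boolean for half a second, with no consumer in this graph.
; Each player's win volume plays the ladder sound, sets P1win or P2win, and clears EndWin on the first Camera_bp1 found.
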(event `self.row1.OnComponentBeginOverlap`
  (params (OverlappedComponent :type "PrimitiveComponent Object Reference") (OtherActor :type "Actor Object Reference") (OtherComp :type "PrimitiveComponent Object Reference") (OtherBodyIndex :type Integer) (bFromSweep :type Boolean) (SweepResult :type "HitResult Structure (by ref)"))
  (cast `/Game/DARKVADAR/darvador_BP` OtherActor)
  (set `self.1st row hit` true)
  (`KismetSystemLibrary.Delay` 0.5)
  (set `self.1st row hit` false))

(event `self.row2.OnComponentBeginOverlap`
  (params (OverlappedComponent :type "PrimitiveComponent Object Reference") (OtherActor :type "Actor Object Reference") (OtherComp :type "PrimitiveComponent Object Reference") (OtherBodyIndex :type Integer) (bFromSweep :type Boolean) (SweepResult :type "HitResult Structure (by ref)"))
  (cast `/Game/DARKVADAR/darvador_BP` OtherActor)
  (set `self.2nd row hit` true)
  (`KismetSystemLibrary.Delay` 0.5)
  (set `self.2nd row hit` false))

(event `self.row3.OnComponentBeginOverlap`
  (params (OverlappedComponent :type "PrimitiveComponent Object Reference") (OtherActor :type "Actor Object Reference") (OtherComp :type "PrimitiveComponent Object Reference") (OtherBodyIndex :type Integer) (bFromSweep :type Boolean) (SweepResult :type "HitResult Structure (by ref)"))
  (cast `/Game/DARKVADAR/darvador_BP` OtherActor)
  (set `self.3rd row hit` true)
  (`KismetSystemLibrary.Delay` 0.5)
  (set `self.3rd row hit` false))

(event `self.row4.OnComponentBeginOverlap`
  (params (OverlappedComponent :type "PrimitiveComponent Object Reference") (OtherActor :type "Actor Object Reference") (OtherComp :type "PrimitiveComponent Object Reference") (OtherBodyIndex :type Integer) (bFromSweep :type Boolean) (SweepResult :type "HitResult Structure (by ref)"))
  (cast `/Game/DARKVADAR/darvador_BP` OtherActor)
  (set `self.4th row hit` true)
  (`KismetSystemLibrary.Delay` 0.5)
  (set `self.4th row hit` false))

(event `self.row 5.OnComponentBeginOverlap`
  (params (OverlappedComponent :type "PrimitiveComponent Object Reference") (OtherActor :type "Actor Object Reference") (OtherComp :type "PrimitiveComponent Object Reference") (OtherBodyIndex :type Integer) (bFromSweep :type Boolean) (SweepResult :type "HitResult Structure (by ref)"))
  (cast `/Game/DARKVADAR/darvador_BP` OtherActor)
  (set `self.5th row` true)
  (`KismetSystemLibrary.Delay` 0.5)
  (set `self.5th row` false))

(event `self.row 6.OnComponentBeginOverlap`
  (params (OverlappedComponent :type "PrimitiveComponent Object Reference") (OtherActor :type "Actor Object Reference") (OtherComp :type "PrimitiveComponent Object Reference") (OtherBodyIndex :type Integer) (bFromSweep :type Boolean) (SweepResult :type "HitResult Structure (by ref)"))
  (cast `/Game/DARKVADAR/darvador_BP` OtherActor)
  (set `self.6th row` true)
  (`KismetSystemLibrary.Delay` 0.5)
  (set `self.6th row` false))

(event `self.row 7.OnComponentBeginOverlap`
  (params (OverlappedComponent :type "PrimitiveComponent Object Reference") (OtherActor :type "Actor Object Reference") (OtherComp :type "PrimitiveComponent Object Reference") (OtherBodyIndex :type Integer) (bFromSweep :type Boolean) (SweepResult :type "HitResult Structure (by ref)"))
  (cast `/Game/DARKVADAR/darvador_BP` OtherActor)
  (set `self.7th row` true)
  (`KismetSystemLibrary.Delay` 0.5)
  (set `self.7th row` false))

(event `self.row 8.OnComponentBeginOverlap`
  (params (OverlappedComponent :type "PrimitiveComponent Object Reference") (OtherActor :type "Actor Object Reference") (OtherComp :type "PrimitiveComponent Object Reference") (OtherBodyIndex :type Integer) (bFromSweep :type Boolean) (SweepResult :type "HitResult Structure (by ref)"))
  (cast `/Game/DARKVADAR/darvador_BP` OtherActor)
  (set `self.8th row` true)
  (`KismetSystemLibrary.Delay` 0.5)
  (set `self.8th row` false))

(event `self.row 9.OnComponentBeginOverlap`
  (params (OverlappedComponent :type "PrimitiveComponent Object Reference") (OtherActor :type "Actor Object Reference") (OtherComp :type "PrimitiveComponent Object Reference") (OtherBodyIndex :type Integer) (bFromSweep :type Boolean) (SweepResult :type "HitResult Structure (by ref)"))
  (cast `/Game/DARKVADAR/darvador_BP` OtherActor)
  (set `self.9th row` true)
  (`KismetSystemLibrary.Delay` 0.5)
  (set `self.9th row` false))

(event `self.Box1.OnComponentBeginOverlap`
  (params (OverlappedComponent :type "PrimitiveComponent Object Reference") (OtherActor :type "Actor Object Reference") (OtherComp :type "PrimitiveComponent Object Reference") (OtherBodyIndex :type Integer) (bFromSweep :type Boolean) (SweepResult :type "HitResult Structure (by ref)"))
  (cast `/Game/DARKVADAR/darvador_BP2` OtherActor)
  (set `self.1st row hit_0` true)
  (`KismetSystemLibrary.Delay` 0.5)
  (set `self.1st row hit_0` false))

(event `self.Box2.OnComponentBeginOverlap`
  (params (OverlappedComponent :type "PrimitiveComponent Object Reference") (OtherActor :type "Actor Object Reference") (OtherComp :type "PrimitiveComponent Object Reference") (OtherBodyIndex :type Integer) (bFromSweep :type Boolean) (SweepResult :type "HitResult Structure (by ref)"))
  (cast `/Game/DARKVADAR/darvador_BP2` OtherActor)
  (set `self.2nd row hit_0` true)
  (`KismetSystemLibrary.Delay` 0.5)
  (set `self.2nd row hit_0` false))

(event `self.Box3.OnComponentBeginOverlap`
  (params (OverlappedComponent :type "PrimitiveComponent Object Reference") (OtherActor :type "Actor Object Reference") (OtherComp :type "PrimitiveComponent Object Reference") (OtherBodyIndex :type Integer) (bFromSweep :type Boolean) (SweepResult :type "HitResult Structure (by ref)"))
  (cast `/Game/DARKVADAR/darvador_BP2` OtherActor)
  (set `self.3rd row hit_0` true)
  (`KismetSystemLibrary.Delay` 0.5)
  (set `self.3rd row hit_0` false))

(event `self.Box4.OnComponentBeginOverlap`
  (params (OverlappedComponent :type "PrimitiveComponent Object Reference") (OtherActor :type "Actor Object Reference") (OtherComp :type "PrimitiveComponent Object Reference") (OtherBodyIndex :type Integer) (bFromSweep :type Boolean) (SweepResult :type "HitResult Structure (by ref)"))
  (cast `/Game/DARKVADAR/darvador_BP2` OtherActor)
  (set `self.4th row hit_0` true)
  (`KismetSystemLibrary.Delay` 0.5)
  (set `self.4th row hit_0` false))

(event `self.Box5.OnComponentBeginOverlap`
  (params (OverlappedComponent :type "PrimitiveComponent Object Reference") (OtherActor :type "Actor Object Reference") (OtherComp :type "PrimitiveComponent Object Reference") (OtherBodyIndex :type Integer) (bFromSweep :type Boolean) (SweepResult :type "HitResult Structure (by ref)"))
  (cast `/Game/DARKVADAR/darvador_BP2` OtherActor)
  (set `self.5th row_0` true)
  (`KismetSystemLibrary.Delay` 0.5)
  (set `self.5th row_0` false))

(event `self.Box6.OnComponentBeginOverlap`
  (params (OverlappedComponent :type "PrimitiveComponent Object Reference") (OtherActor :type "Actor Object Reference") (OtherComp :type "PrimitiveComponent Object Reference") (OtherBodyIndex :type Integer) (bFromSweep :type Boolean) (SweepResult :type "HitResult Structure (by ref)"))
  (cast `/Game/DARKVADAR/darvador_BP2` OtherActor)
  (set `self.6th row_0` true)
  (`KismetSystemLibrary.Delay` 0.5)
  (set `self.6th row_0` false))

(event `self.Box7.OnComponentBeginOverlap`
  (params (OverlappedComponent :type "PrimitiveComponent Object Reference") (OtherActor :type "Actor Object Reference") (OtherComp :type "PrimitiveComponent Object Reference") (OtherBodyIndex :type Integer) (bFromSweep :type Boolean) (SweepResult :type "HitResult Structure (by ref)"))
  (cast `/Game/DARKVADAR/darvador_BP2` OtherActor)
  (set `self.7th row_0` true)
  (`KismetSystemLibrary.Delay` 0.5)
  (set `self.7th row_0` false))

(event `self.Box8.OnComponentBeginOverlap`
  (params (OverlappedComponent :type "PrimitiveComponent Object Reference") (OtherActor :type "Actor Object Reference") (OtherComp :type "PrimitiveComponent Object Reference") (OtherBodyIndex :type Integer) (bFromSweep :type Boolean) (SweepResult :type "HitResult Structure (by ref)"))
  (cast `/Game/DARKVADAR/darvador_BP2` OtherActor)
  (set `self.8th row_0` true)
  (`KismetSystemLibrary.Delay` 0.5)
  (set `self.8th row_0` false))

(event `self.Box9.OnComponentBeginOverlap`
  (params (OverlappedComponent :type "PrimitiveComponent Object Reference") (OtherActor :type "Actor Object Reference") (OtherComp :type "PrimitiveComponent Object Reference") (OtherBodyIndex :type Integer) (bFromSweep :type Boolean) (SweepResult :type "HitResult Structure (by ref)"))
  (cast `/Game/DARKVADAR/darvador_BP2` OtherActor)
  (set `self.9th row_0` true)
  (`KismetSystemLibrary.Delay` 0.5)
  (set `self.9th row_0` false))

(event `self.win collision.OnComponentBeginOverlap`
  (params (OverlappedComponent :type "PrimitiveComponent Object Reference") (OtherActor :type "Actor Object Reference") (OtherComp :type "PrimitiveComponent Object Reference") (OtherBodyIndex :type Integer) (bFromSweep :type Boolean) (SweepResult :type "HitResult Structure (by ref)"))
  ;[1 1 1] win game
  (cast `/Game/DARKVADAR/darvador_BP` OtherActor)
  (`GameplayStatics.PlaySound2D` "/Game/ladder_sound.ladder_sound" 1.5 1.0 0.0 null null)
  (set `self.p1win` true)
  (bind _outactors (`GameplayStatics.GetAllActorsOfClass` "/Game/camera_bp1.camera_bp1_C"))
  (set `/Game/camera_bp1.end win` false (`|GetArrayItem` _outactors)))

(event `self.win collion 2.OnComponentBeginOverlap`
  (params (OverlappedComponent :type "PrimitiveComponent Object Reference") (OtherActor :type "Actor Object Reference") (OtherComp :type "PrimitiveComponent Object Reference") (OtherBodyIndex :type Integer) (bFromSweep :type Boolean) (SweepResult :type "HitResult Structure (by ref)"))
  ;[1 1 1] win game
  (cast `/Game/DARKVADAR/darvador_BP2` OtherActor)
  (`GameplayStatics.PlaySound2D` "/Game/ladder_sound.ladder_sound" 1.5 1.0 0.0 null null)
  (set `self.p2win` true)
  (bind _outactors (`GameplayStatics.GetAllActorsOfClass` "/Game/camera_bp1.camera_bp1_C"))
  (set `/Game/camera_bp1.end win` false (`|GetArrayItem` _outactors)))

(fn `UserConstructionScript`)