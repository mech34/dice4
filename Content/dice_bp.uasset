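; Physics die actor that rolls when Camera_bp1's DiceRoleOhYea flag is set and works out its score.
; Tick releases it with gravity and random angular impulses, then lifts it back spinning after a result.
; Six boxes flag floor overlaps; once angular velocity is zero, the flag sets ScoreXx, highlights the material and plays a score-pitched sound.
; Another box plays the floor-impact sound, and falling too low teleports the die back up.
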(event `self.ReceiveTick`
  (params (DeltaSeconds :type "Float (single-precision)"))
  (bind _staticmesh_dice (`self.StaticMesh-dice`))
  (bind (_returnvalue_x _returnvalue_y _returnvalue_z) (`KismetMathLibrary.BreakVector` (`SceneComponent.K2_GetComponentLocation` (`self.StaticMesh-dice`))))
  (`|ExecutionSequence` :!label _label
    (:`then_0`
      (if (== (`self.reset role`) true)
        (bind _output (`|GetArrayItem` (stale _outactors)))
        (if (== (`/Game/camera_bp1.dice role oh yea` _output) true)
          (set `self.restart dice calculation` true)
          (`PrimitiveComponent.SetEnableGravity` _staticmesh_dice true :!label _label_2)
          (`KismetSystemLibrary.Delay` 0.1)
          (set `self.reset role` false)
          (`PrimitiveComponent.AddAngularImpulseInDegrees` _staticmesh_dice (`KismetMathLibrary.MakeVector` (`KismetMathLibrary.RandomFloatInRange` 70.0 360.0) (`KismetMathLibrary.RandomFloatInRange` 60.0 360.0) (`KismetMathLibrary.RandomFloatInRange` 80.0 360.0)) "None" true))
        (else
          (bind _outactors (`GameplayStatics.GetAllActorsOfClass` "/Game/camera_bp1.camera_bp1_C"))
          (if (== (`/Game/camera_bp1.dice role oh yea` _output) true)
            (`/Engine/EditorBlueprintResources/StandardMacros.DoOnce` false
              (:`Completed`
                (set `self.restart dice calculation` true)
                (goto _label_2)))
            (else
              (if (== (`self.dice stopped`) true)
                (`KismetSystemLibrary.Delay` 2.0)
                (`PrimitiveComponent.SetEnableGravity` (`self.StaticMesh-dice`) false)
                (`KismetSystemLibrary.MoveComponentTo` (`self.StaticMesh-dice`) (-70.0 0.0 1884.0) (`KismetMathLibrary.MakeRotator` (`KismetMathLibrary.RandomFloatInRange` 80.0 500.0) (`KismetMathLibrary.RandomFloatInRange` 90.0 500.0) (`KismetMathLibrary.RandomFloatInRange` 95.0 500.0)) false false 0.3)
                (`KismetSystemLibrary.Delay` 0.1)
                (set `self.reset role` true)
                (`MeshComponent.SetScalarParameterValueOnMaterials` (`self.StaticMesh-dice`) "dice shine" 0.0)
                (`MeshComponent.SetVectorParameterValueOnMaterials` (`self.StaticMesh-dice`) "colour white" (1.0 1.0 1.0))
                (else
                  (`/Engine/EditorBlueprintResources/StandardMacros.DoOnce` false
                    (:`Completed`
                      (set `self.restart dice calculation` true)))))
              (`PrimitiveComponent.AddAngularImpulseInDegrees` _staticmesh_dice (`KismetMathLibrary.MakeVector` (`KismetMathLibrary.RandomFloatInRange` 240.0 450.0) (`KismetMathLibrary.RandomFloatInRange` 200.0 450.0) (`KismetMathLibrary.RandomFloatInRange` 250.0 450.0)) "None" true))))))
    (:`then_1`
      (if (== (== (`PrimitiveComponent.GetPhysicsAngularVelocityInDegrees` (`self.StaticMesh-dice`) "None") (0.0 0.0 0.0) :`ErrorTolerance` 0.0) true)
        (`|ExecutionSequence`
          (:`then_0`
            (if (== (`self.1`) true)
              ;[1 1 1] ?
              (if (== (`self.restart dice calculation`) true)
                (set `self.2` false)
                (set `self.3` false)
                (set `self.4` false)
                (set `self.5` false)
                (set `self.6` false)
                (set `self.score xx` 1.0)
                (set `self.restart dice calculation` false)
                (`MeshComponent.SetVectorParameterValueOnMaterials` (`self.StaticMesh-dice`) "dicecolour_b" (1.0 0.27 0.0) :!label _label_3)
                (`MeshComponent.SetScalarParameterValueOnMaterials` (`self.StaticMesh-dice`) "dice shine" 30.0)
                (`MeshComponent.SetVectorParameterValueOnMaterials` (`self.StaticMesh-dice`) "colour white" (0.5 0.5 0.5))
                (`|ExecutionSequence`
                  (:`then_0`
                    (`/Engine/EditorBlueprintResources/StandardMacros.DoOnce` false :!label _label_4
                      (:`Completed`
                        (`GameplayStatics.PlaySound2D` "/Game/Arcade_GameStart.Arcade_GameStart" 0.5 (* (`self.score xx`) 0.2) 0.0 null null)
                        (set `self.1` false)
                        (set `self.2` false)
                        (set `self.3` false)
                        (set `self.4` false)
                        (set `self.5` false)
                        (set `self.6` false)
                        (set `self.dice stopped` true))))
                  (:`then_1`
                    (if (== (`self.dice stopped`) true)
                      (goto _label_4 :!via `Reset`)))))))
          (:`then_1`
            (if (== (`self.2`) true)
              (if (== (`self.restart dice calculation`) true)
                (set `self.1` false)
                (set `self.3` false)
                (set `self.4` false)
                (set `self.5` false)
                (set `self.6` false)
                (set `self.score xx` 2.0)
                (set `self.restart dice calculation` false)
                (goto _label_3))))
          (:`then_2`
            (if (== (`self.3`) true)
              (if (== (`self.restart dice calculation`) true)
                (set `self.1` false)
                (set `self.2` false)
                (set `self.4` false)
                (set `self.5` false)
                (set `self.6` false)
                (set `self.score xx` 3.0)
                (set `self.restart dice calculation` false)
                (goto _label_3))))
          (:`then_3`
            (if (== (`self.4`) true)
              (if (== (`self.restart dice calculation`) true)
                (set `self.1` false)
                (set `self.2` false)
                (set `self.3` false)
                (set `self.5` false)
                (set `self.6` false)
                (set `self.score xx` 4.0)
                (set `self.restart dice calculation` false)
                (goto _label_3))))
          (:`then_4`
            (if (== (`self.5`) true)
              (if (== (`self.restart dice calculation`) true)
                (set `self.1` false)
                (set `self.2` false)
                (set `self.4` false)
                (set `self.3` false)
                (set `self.6` false)
                (set `self.score xx` 5.0)
                (set `self.restart dice calculation` false)
                (goto _label_3))))
          (:`then_5`
            (if (== (`self.6`) true)
              (if (== (`self.restart dice calculation`) true)
                (set `self.1` false)
                (set `self.2` false)
                (set `self.4` false)
                (set `self.5` false)
                (set `self.3` false)
                (set `self.score xx` 6.0)
                (set `self.restart dice calculation` false)
                (goto _label_3)))))))
    (:`then_2`
      (if (<= _returnvalue_z -150.0)
        (`self.K2_TeleportTo` (-70.0 120.0 1884.0))
        (goto _label)))))

(event `self.Box1.OnComponentBeginOverlap`
  (params (OverlappedComponent :type "PrimitiveComponent Object Reference") (OtherActor :type "Actor Object Reference") (OtherComp :type "PrimitiveComponent Object Reference") (OtherBodyIndex :type Integer) (bFromSweep :type Boolean) (SweepResult :type "HitResult Structure (by ref)"))
  (cast `/Game/floor_bp` OtherActor)
  (set `self.1` true))

(event `self.Box2.OnComponentBeginOverlap`
  (params (OverlappedComponent :type "PrimitiveComponent Object Reference") (OtherActor :type "Actor Object Reference") (OtherComp :type "PrimitiveComponent Object Reference") (OtherBodyIndex :type Integer) (bFromSweep :type Boolean) (SweepResult :type "HitResult Structure (by ref)"))
  (cast `/Game/floor_bp` OtherActor)
  (set `self.2` true))

(event `self.Box3.OnComponentBeginOverlap`
  (params (OverlappedComponent :type "PrimitiveComponent Object Reference") (OtherActor :type "Actor Object Reference") (OtherComp :type "PrimitiveComponent Object Reference") (OtherBodyIndex :type Integer) (bFromSweep :type Boolean) (SweepResult :type "HitResult Structure (by ref)"))
  (cast `/Game/floor_bp` OtherActor)
  (set `self.3` true))

(event `self.Box4.OnComponentBeginOverlap`
  (params (OverlappedComponent :type "PrimitiveComponent Object Reference") (OtherActor :type "Actor Object Reference") (OtherComp :type "PrimitiveComponent Object Reference") (OtherBodyIndex :type Integer) (bFromSweep :type Boolean) (SweepResult :type "HitResult Structure (by ref)"))
  (cast `/Game/floor_bp` OtherActor)
  (set `self.4` true))

(event `self.Box5.OnComponentBeginOverlap`
  (params (OverlappedComponent :type "PrimitiveComponent Object Reference") (OtherActor :type "Actor Object Reference") (OtherComp :type "PrimitiveComponent Object Reference") (OtherBodyIndex :type Integer) (bFromSweep :type Boolean) (SweepResult :type "HitResult Structure (by ref)"))
  (cast `/Game/floor_bp` OtherActor)
  (set `self.5` true))

(event `self.Box6.OnComponentBeginOverlap`
  (params (OverlappedComponent :type "PrimitiveComponent Object Reference") (OtherActor :type "Actor Object Reference") (OtherComp :type "PrimitiveComponent Object Reference") (OtherBodyIndex :type Integer) (bFromSweep :type Boolean) (SweepResult :type "HitResult Structure (by ref)"))
  (cast `/Game/floor_bp` OtherActor)
  (set `self.6` true))

(event `self.sound box.OnComponentBeginOverlap`
  (params (OverlappedComponent :type "PrimitiveComponent Object Reference") (OtherActor :type "Actor Object Reference") (OtherComp :type "PrimitiveComponent Object Reference") (OtherBodyIndex :type Integer) (bFromSweep :type Boolean) (SweepResult :type "HitResult Structure (by ref)"))
  (cast `/Game/floor_bp` OtherActor)
  (`GameplayStatics.PlaySound2D` "/Game/Pinball_BallDropFromSlide.Pinball_BallDropFromSlide" 0.5 0.3 0.0 null null))

(fn `UserConstructionScript`)