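; Animated "Snake and Dice" title Blueprint that plays its text intro on BeginPlay and replays it on player turns.
; Chained MoveComponentTo calls slide and tilt the Snake, And and Dice components into place, activating a sigil FX.
; Tick polls Camera_bp1's P1Turn and P2Turn, using DoOnce gates to slide Snake and Dice outward, then loop back into the intro.
; Tick also randomizes the point light's intensity for flicker.
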(event `self.ReceiveBeginPlay`
  (bind _snake (`self.snake`))
  (bind _dice (`self.dice`))
  (bind _and (`self.and`))
  (`|ExecutionSequence` :!label _label
    (:`then_0`
      (`KismetSystemLibrary.MoveComponentTo` _snake (-250.0 0.0 0.0) (struct) true true 0.8)
      (`KismetSystemLibrary.MoveComponentTo` _snake (-250.0 0.0 0.0) (struct :`Roll` 10.0) true true 0.8)
      (set `self.play1` false)
      (set `self.play2` false))
    (:`then_1`
      (`KismetSystemLibrary.MoveComponentTo` _dice (200.0 0.0 0.0) (struct) true true 0.8)
      (`KismetSystemLibrary.MoveComponentTo` _dice (200.0 0.0 0.0) (struct :`Roll` 10.0) true true 0.8))
    (:`then_2`
      (`KismetSystemLibrary.Delay` 0.2)
      (`KismetSystemLibrary.MoveComponentTo` _and (0.0 0.0 0.0) (struct) true true 0.4)
      (`KismetSystemLibrary.Delay` 0.2)
      (`ActorComponent.SetActive` (`self.FX_Sigil_03`) true false)
      (`KismetSystemLibrary.MoveComponentTo` _and (0.0 0.0 0.0) (struct :`Roll` 30.0) true true 1.0))))

(event `self.ReceiveTick`
  (params (DeltaSeconds :type "Float (single-precision)"))
  (`|ExecutionSequence`
    (:`then_0`
      (bind _outactors (`GameplayStatics.GetAllActorsOfClass` "/Game/camera_bp1.camera_bp1_C"))
      (`|ExecutionSequence`
        (:`then_0`
          (bind _output (`|GetArrayItem` _outactors))
          (if (== (`/Game/camera_bp1.p1 turn ` _output) true)
            (set `self.play1` true)
            (`/Engine/EditorBlueprintResources/StandardMacros.DoOnce` false :!label _label_2
              (:`Completed`
                (`|ExecutionSequence`
                  (:`then_0`
                    (`KismetSystemLibrary.MoveComponentTo` (`self.snake`) (-900.0 0.0 0.0) (struct) true true 0.5 :!label _label_3)
                    (goto _label))
                  (:`then_1`
                    (`KismetSystemLibrary.MoveComponentTo` (`self.dice`) (900.0 0.0 0.0) (struct) true true 0.5 :!label _label_4)
                    (`ActorComponent.SetActive` (`self.FX_Sigil_03`) false false)
                    (goto _label)))))))
        (:`then_1`
          (if (== (`self.play1`) false)
            (goto _label_2 :!via `Reset`)))
        (:`then_2`
          (if (== (`/Game/camera_bp1.p2 turn` _output) true)
            (set `self.play2` true)
            (`/Engine/EditorBlueprintResources/StandardMacros.DoOnce` false :!label _label_5
              (:`Completed`
                (`|ExecutionSequence`
                  (:`then_0`
                    (goto _label_3))
                  (:`then_1`
                    (goto _label_4)))))))
        (:`then_3`
          (if (== (`self.play2`) false)
            (goto _label_5 :!via `Reset`)))))
    (:`then_1`
      (`LightComponent.SetIntensity` (`self.PointLight`) (`KismetMathLibrary.RandomFloatInRange` 1.0 15000.0)))))

(fn `UserConstructionScript`)